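; Spell system that holds a caster's spell list, cycles the selection with wraparound and casts the current spell.
; Setup finds or spawns the Spell_Database, which AddSpell copies entries from into a list with a parallel cooldown array.
; Cast, gated by cooldown and cast time, spawns a Spell_Base actor, activates it, attaches it to the caster mesh, plays a montage and sets any target.
; Tick counts down both timers.
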(fn SelectNext
  (if (> (+ (Variables|Default|GetCurrentSpell) 1) (Utilities|Array|LastIndex (Variables|Default|GetAvailable_Spells))) ; if we reached end of the list, go to beginning, otherwise select the next spell
    (Variables|Default|SetCurrentSpell 0)
    (else
      (Variables|Default|SetCurrentSpell (+ (Variables|Default|GetCurrentSpell) 1)))))

(fn SelectPrevious
  (if (< (- (Variables|Default|GetCurrentSpell) 1) 0) ; if we reached the start then go to the end, or pick previous spell
    (Variables|Default|SetCurrentSpell (Utilities|Array|LastIndex (Variables|Default|GetAvailable_Spells)))
    (else
      (Variables|Default|SetCurrentSpell (- (Variables|Default|GetCurrentSpell) 1)))))

(fn Cast
  (params (Caster :type Pawn%20Object%20Reference) (Caster_Mesh :type Skeletal%20Mesh%20Component%20Object%20Reference) (CastRotation :type Rotator) (CastPositionOffset :type Vector) (SpellTarget :type Actor%20Object%20Reference))
  (Variables|Default|SetSuccess false)
  (Variables|Default|SetCaster Caster)
  (Variables|Default|SetAnimMesh Caster_Mesh)
  (Variables|Default|SetRotator CastRotation)
  (if (and (not (Variables|Default|GetCasting)) (not (> (Utilities|Array|Get(acopy) (Variables|Default|GetCooldowns) (Variables|Default|GetCurrentSpell)) 0.0))) ; If we are NOT casting and if the current spell is NOT on Cooldown
    (Variables|Default|SetCasting true)
    (bind _current_spell (CallFunction|GetCurrentSpell))
    (LocalVariables|Settmp_CurrentSpell _current_spell)
    (Utilities|FlowControl|Sequence
      (:then_0
        ;[1 1 1] Spawn the spell and set it on cooldown
        (Utilities|Array|SetArrayElem (Variables|Default|GetCooldowns) (Variables|Default|GetCurrentSpell) (.Cooldown (Utilities|Struct|BreakSpellStruct (LocalVariables|Gettmp_CurrentSpell))))
        (Variables|Default|SetCastTime (.CastTime (Utilities|Struct|BreakSpellStruct (LocalVariables|Gettmp_CurrentSpell))))
        (bind _returnvalue (Game|SpawnActorfromClass (.Spell_ParticleBP (Utilities|Struct|BreakSpellStruct (LocalVariables|Gettmp_CurrentSpell))) (Math|Transform|MakeTransform (+ (Transformation|GetActorLocation (Variables|Default|GetCaster)) (Math|Vector|RotateVector CastPositionOffset (Variables|Default|GetRotator))) (Variables|Default|GetRotator)) "AlwaysSpawn" 0 0)) ; Spawn projectile
        (bind _asspell_base (Utilities|Casting|CastToSpell_Base _returnvalue)
          (:then
            (Variables|Default|SetCurrent%20Spell%20Object _asspell_base))
          (:CastFailed
            (return (Variables|Default|GetSuccess) (LocalVariables|Gettmp_CurrentSpell)))))
      (:then_1
        ;[1 1 1] Active the spell and attach the newly spawned spell to the Caster
        (Default|Cast (Variables|Default|GetCurrent%20Spell%20Object) (LocalVariables|Gettmp_CurrentSpell))
        (if (Utilities|IsValid (Variables|Default|GetAnimMesh))
          (Class|Actor|AttachRootComponentto (Variables|Default|GetCurrent%20Spell%20Object) (Variables|Default|GetAnimMesh) "None" "KeepWorldPosition" false) ; attach the spell to the player durring cast
        ))
      (:then_2
        ;[1 1 1] Set the spells position and play the casting animation
        (if (Utilities|IsValid (Variables|Default|GetAnimMesh)) ; is there a mesh to animate?
          (Animation|Montage|MontagePlay (Components|SkeletalMesh|GetAnimInstance (Variables|Default|GetAnimMesh)) (.Animation (Utilities|Struct|BreakSpellStruct (LocalVariables|Gettmp_CurrentSpell))) 1.0) ; Play animation on arm mesh
        ))
      (:then_3
        ;[1 1 1] Set the target for the spell if there is one, and return true if a spell object exists (spell has been casted)
        (if (Utilities|IsValid SpellTarget)
          (Variables|/Game/Blueprints/SpellSystem/Spells/Spell_Base.Spell_Base_C|SetTarget (Variables|Default|GetCurrent%20Spell%20Object) SpellTarget))
        (Variables|Default|SetSuccess (Utilities|IsValid (Variables|Default|GetCurrent%20Spell%20Object)))
        (return (Variables|Default|GetSuccess) (LocalVariables|Gettmp_CurrentSpell))))
    (else
      (return (Variables|Default|GetSuccess) (LocalVariables|Gettmp_CurrentSpell)))))

(fn GetPower
  (bind _current_spell (CallFunction|GetCurrentSpell))
  (return (.Power (Utilities|Struct|BreakSpellStruct _current_spell))))

(fn GetManaCost
  (bind _current_spell (CallFunction|GetCurrentSpell))
  (return (.Mana (Utilities|Struct|BreakSpellStruct _current_spell))))

(fn GetType
  (bind _current_spell (CallFunction|GetCurrentSpell))
  (return (.Type (Utilities|Struct|BreakSpellStruct _current_spell))))

(fn GetCurrentSpell
  (return (Utilities|Array|Get(acopy) (Variables|Default|GetAvailable_Spells) (Variables|Default|GetCurrentSpell))))

(fn Tick
  (params (Delta%20Time :type Float%20%28single-precision%29))
  (Utilities|FlowControl|Sequence
    (:then_0
      (for (_array_element _array_index) (Variables|Default|GetCooldowns)
        (if (> _array_element 0.0)
          (Utilities|Array|SetArrayElem (Variables|Default|GetCooldowns) _array_index (- _array_element Delta%20Time)))))
    (:then_1
      (if (> (Variables|Default|GetCastTime) 0.0)
        (Variables|Default|SetCastTime (- (Variables|Default|GetCastTime) Delta%20Time))
        (else
          (Variables|Default|SetCasting false))))))

(fn AddSpell
  (params (ID :type Integer))
  (Utilities|Array|Add (Variables|Default|GetAvailable_Spells) (Utilities|Array|Get(acopy) (Variables|/Game/Blueprints/SpellSystem/Spell_Database.Spell_Database_C|GetSpells (Variables|Default|GetSpell_Database)) ID))
  (Utilities|Array|Add (Variables|Default|GetCooldowns) 0.0))

(fn Setup
  ;[1 1 1] Get reference to spell database if it exists within the world, if it doesn;t spawn it.
  (bind _outactors (Actor|GetAllActorsOfClass "/Game/Blueprints/SpellSystem/Spell_Database.Spell_Database_C"))
  (if (== (Utilities|Array|LastIndex _outactors) -1)
    (bind _returnvalue (Game|SpawnActorfromClass (Variables|Default|GetSpell_Database_Class) (Math|Transform|MakeTransform "0, 0, 0") "AlwaysSpawn" 0 0))
    (bind _asspell_database (Utilities|Casting|CastToSpell_Database _returnvalue))
    (Variables|Default|SetSpell_Database _asspell_database)
    (else
      (bind _asspell_database_2 (Utilities|Casting|CastToSpell_Database (Utilities|Array|Get(acopy) _outactors)))
      (Variables|Default|SetSpell_Database _asspell_database_2))))

(fn RemoveSpell
  (params (ID :type Integer))
  (Utilities|Array|RemoveIndex (Variables|Default|GetAvailable_Spells) ID)
  (Utilities|Array|RemoveIndex (Variables|Default|GetCooldowns) ID))