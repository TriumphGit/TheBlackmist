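; Follower_AI_CON2 is an AI controller that sets up and starts the behavior of a follower pawn.
; On BeginPlay it initializes FollowerBlackboard2 and stores the pawn's starting location as HomeLocation.
; It then sets hardcoded radius variables for two aggro ranges, shooting and pursuit before running FollowerBT2.
; It has no Tick logic, and nothing in this graph reads those radii.
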(event `/Game/Blueprints/AI/Follower_AI_CON.ReceiveBeginPlay`
  (`self.UseBlackboard` "/Game/Blueprints/AI/FollowerBlackboard2.FollowerBlackboard2")
  (`BlackboardComponent.SetValueAsVector` (`AIBlueprintHelperLibrary.GetBlackboard` self) (`self.HomeLocation`) (`self.K2_GetActorLocation` (`self.K2_GetPawn`)))
  (`|ExecutionSequence`
    (:`then_0`
      (set `self.RAggro1` 1200.0))
    (:`then_1`
      (set `self.RShoot` 900.0))
    (:`then_2`
      (set `self.RAggro2` 1800.0))
    (:`then_3`
      (set `self.RPursuit` 2400.0))
    (:`then_4`
      (`self.RunBehaviorTree` "/Game/Blueprints/AI/FollowerBT2.FollowerBT2"))))

(event `self.ReceiveTick`
  (params (DeltaSeconds :type "Float (single-precision)")))

(fn `UserConstructionScript`)