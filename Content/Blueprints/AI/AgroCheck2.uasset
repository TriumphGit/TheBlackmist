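; Behavior tree service that runs aggro detection for AI_Characters controlled by Follower_AI_CON2.
; Each tick it sphere-traces the controller's aggro radius, ignoring all AI_Characters, then line-traces on the Camera channel to each hit.
; Visible hits set TargetToFollow and TargetLocation, while blocked ones clear TargetToFollow, so the last hit processed decides the target.
; Dead characters skip detection and have WantsFire cleared.
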(event `self.ReceiveTick`
  (params (OwnerActor :type "Actor Object Reference") (DeltaSeconds :type "Float (single-precision)"))
  (bind _returnvalue (`Controller.K2_GetPawn` (`self.AI_CON_Ref`)))
  (bind _returnvalue_2 (`Actor.K2_GetActorLocation` _returnvalue))
  (if (not (!= (`self.AI_CON_Ref`) null))
    (bind _asfollower_ai_con2 (cast `/Game/Blueprints/AI/Follower_AI_CON2` OwnerActor))
    (set `self.AI_CON_Ref` _asfollower_ai_con2))
  (bind _outactors (`GameplayStatics.GetAllActorsOfClass` "/Game/Blueprints/AI/AI_Character.AI_Character_C"))
  (bind _asai_character (cast `/Game/Blueprints/AI/AI_Character` _returnvalue))
  (if (`/Game/Blueprints/AI/AI_Character.IsDead` _asai_character)
    (set `/Game/Blueprints/AI/AI_Character.WantsFire` false _asai_character)
    (else
      (set `self.MyLocation` _returnvalue_2)
      (bind _outhits (`KismetSystemLibrary.SphereTraceMultiForObjects` _returnvalue_2 (+ _returnvalue_2 (0.0 0.0 15.0)) (`/Game/Blueprints/AI/Follower_AI_CON2.RAggro1` _asfollower_ai_con2) (`self.DesiredObjectTypes`) false _outactors "ForDuration"))
      (for _array_element _outhits
        (bind (_bblockinghit _binitialoverlap _time _location _impactpoint _normal _impactnormal _physmat _hitactor) (`GameplayStatics.BreakHitResult` _array_element))
        (bind _outhit (`KismetSystemLibrary.LineTraceSingle` (`self.MyLocation`) (`Actor.K2_GetActorLocation` _hitactor) "TraceTypeQuery2" false _outactors "ForDuration"))
        (bind (_bblockinghit_2 _binitialoverlap_2 _time_2 _location_2 _impactpoint_2 _normal_2 _impactnormal_2 _physmat_2 _hitactor_2) (`GameplayStatics.BreakHitResult` _outhit))
        (if (== _hitactor_2 _hitactor)
          (`BTFunctionLibrary.SetBlackboardValueAsObject` (`self.TargetToFollow`) _hitactor_2)
          (`BTFunctionLibrary.SetBlackboardValueAsVector` (`self.TargetLocation`) (`Actor.K2_GetActorLocation` _hitactor_2))
          (else
            (`BTFunctionLibrary.SetBlackboardValueAsObject` (`self.TargetToFollow`))))))))