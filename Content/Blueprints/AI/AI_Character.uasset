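; AI-controlled NPC character that shoots at the player and leaves a blood pool when killed.
; Tick checks health; while alive with WantsFire set, it turns to the player and, after a short delay, traces from the muzzle toward a random reachable point near their neck.
; Player hits only spawn blood particles.
; At zero health, it once traces to the floor, waits, then spawns a temporary blood pool under the spine, scaled by a timeline.
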(event `self.ReceiveBeginPlay`
  (`|ExecutionSequence`
    (:`then_0`
      (set `self.NPC_Health` 100.0))))

(event `self.ReceiveTick`
  (params (DeltaSeconds :type "Float (single-precision)"))
  (bind _returnvalue (`GameplayStatics.GetPlayerCharacter` 0))
  (bind _returnvalue_2 (`self.K2_GetActorLocation`))
  (bind _aiweapon (`self.AIWeapon`))
  (if (<= (`self.NPC_Health`) 0.0)
    (set `self.IsDead` true)
    (`/Engine/EditorBlueprintResources/StandardMacros.DoOnce` false
      (:`Completed`
        (bind _outhit (`KismetSystemLibrary.LineTraceSingle` _returnvalue_2 (- _returnvalue_2 (0.0 0.0 1000.0)) "TraceTypeQuery1"))
        (`KismetSystemLibrary.Delay` 6.0)
        (bind _returnvalue_3 (`|SpawnActorFromClass` "/Game/Effects/Blood/Blueprints/BP_BloodPool_Actor.BP_BloodPool_Actor_C" (`KismetMathLibrary.MakeTransform` (`KismetMathLibrary.MakeVector` (.x (`SceneComponent.GetSocketLocation` (`self.Mesh`) "spine_02")) (.y (`SceneComponent.GetSocketLocation` (`self.Mesh`) "spine_02")) (+ (.z (`.Location` (`GameplayStatics.BreakHitResult` _outhit))) 0.5))) "Undefined" "OverrideRootScale"))
        (`self.SetLifeSpan` _returnvalue_3 30.0)
        (bind (_direction _scale) (`Timeline|Timeline_0`)
          (:`Update`
            (`self.SetActorScale3D` _returnvalue_3 _scale)))))
    (else
      (`|ExecutionSequence`
        (:`then_1`
          (if (`self.WantsFire`)
            (bind _asthird_person_character (cast `/Game/Character/ThirdPersonCharacter/ThirdPersonCharacter` _returnvalue))
            (`self.SetActorRotation` (`KismetMathLibrary.Conv_VectorToRotator` (`KismetMathLibrary.GreaterGreater_VectorRotator` (`KismetMathLibrary.Normal` (* (- (`self.K2_GetActorLocation` _returnvalue) (`self.K2_GetActorLocation`)) (1.0 1.0 0.0))))))
            (`KismetSystemLibrary.Delay` 0.23)
            (bind _outhit_2 (`KismetSystemLibrary.LineTraceSingle` :`Start` (`SceneComponent.GetSocketLocation` _aiweapon "MuzzleFlash") :`End` (`NavigationSystem.GetRandomReachablePointInRadius` (`SceneComponent.GetSocketLocation` (`Character.Mesh` _asthird_person_character) "NeckSocket") 200.0) :`TraceChannel` "TraceTypeQuery1" :`bIgnoreSelf` false))
            (bind (_bblockinghit _binitialoverlap _time _location _impactpoint _normal _impactnormal _physmat _hitactor) (`GameplayStatics.BreakHitResult` _outhit_2))
            (if (== _returnvalue _hitactor)
              (`GameplayStatics.SpawnEmitterAtLocation` "/Game/Effects/Blood/Particles/PS_Blood_BulletHit.PS_Blood_BulletHit" _location (`SceneComponent.GetSocketRotation` _aiweapon "AmmoEject") false))))))))

(fn `UserConstructionScript`)