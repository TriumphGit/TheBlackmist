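; CloseEnough2 is a behavior tree decorator condition for follower AI run by Follower_AI_CON2.
; It passes when the controlled AI_Character is not dead and its distance to the TargetToFollow blackboard actor is at least AcceptableDistance.
; AcceptableDistance is reset to zero on every check, so the distance test always passes and the living state effectively decides the result.
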(fn `PerformConditionCheck`
  (params (OwnerActor :type "Actor Object Reference"))
  (returns (ReturnValue :type Boolean))
  (bind _returnvalue (`Controller.K2_GetPawn` (`self.AI_CON_Ref`)))
  (bind _asfollower_ai_con2 (cast `/Game/Blueprints/AI/Follower_AI_CON2` OwnerActor))
  (set `self.AI_CON_Ref` _asfollower_ai_con2)
  (bind _output_get (set `self.AcceptableDistance` 0.0))
  (bind _asai_character (cast `/Game/Blueprints/AI/AI_Character` _returnvalue))
  (return (and (!= (`/Game/Blueprints/AI/AI_Character.IsDead` _asai_character) true) (>= (`KismetMathLibrary.VSize` (- (`Actor.K2_GetActorLocation` (`BTFunctionLibrary.GetBlackboardValueAsActor` (`self.TargetToFollow`))) (`Actor.K2_GetActorLocation` _returnvalue))) _output_get))))