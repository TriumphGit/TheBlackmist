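; RapidMoveTo is a behavior tree task that moves an AI follower to the blackboard's TargetToFollow actor.
; On execute it caches the Follower_AI_CON2 controller, then stops the AI_Character firing, flags it as moving and sets a fixed AI speed.
; AIMoveTo uses the controller's RShoot as acceptance radius and finishes the task only on success, with no failure handling.
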(event `self.ReceiveExecute`
  (params (OwnerActor :type "Actor Object Reference"))
  (bind _returnvalue (`Controller.K2_GetPawn` (`self.AI_CON_Ref`)))
  (if (not (!= (`self.AI_CON_Ref`) null))
    (bind _asfollower_ai_con2 (cast `/Game/Blueprints/AI/Follower_AI_CON2` OwnerActor))
    (set `self.AI_CON_Ref` _asfollower_ai_con2))
  (bind _asai_character (cast `/Game/Blueprints/AI/AI_Character` _returnvalue))
  (set `/Game/Blueprints/AI/AI_Character.WantsFire` false _asai_character)
  (set `/Game/Blueprints/AI/AI_Character.IsMoving` true _asai_character)
  (set `/Game/Blueprints/AI/AI_Character.AISpeed` 50.0 _asai_character)
  (`|AIMoveTo` _returnvalue (0.0 0.0 0.0) (`BTFunctionLibrary.GetBlackboardValueAsActor` (`self.TargetToFollow`)) (`/Game/Blueprints/AI/Follower_AI_CON2.RShoot` _asfollower_ai_con2)
    (:`OnSuccess`
      (`self.FinishExecute` true))))