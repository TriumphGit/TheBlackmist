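; TryFind is a Behavior Tree task that sends an AI character to search near the blackboard point LSPoint.
; It caches the Follower_AI_CON2 controller on first run, then clears WantsFire and sets IsMoving on the controlled AI_Character.
; AIMoveTo heads to a random reachable point close to LSPoint, and the move result finishes the task as success or failure.
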(event `self.ReceiveExecute`
  (params (OwnerActor :type "Actor Object Reference"))
  (bind _returnvalue (`Controller.K2_GetPawn` (`self.AI_CON_Ref`)))
  (if (not (!= (`self.AI_CON_Ref`) null))
    (bind _asfollower_ai_con2 (cast `/Game/Blueprints/AI/Follower_AI_CON2` OwnerActor))
    (set `self.AI_CON_Ref` _asfollower_ai_con2))
  (bind _asai_character (cast `/Game/Blueprints/AI/AI_Character` _returnvalue))
  (set `/Game/Blueprints/AI/AI_Character.WantsFire` false _asai_character)
  (set `/Game/Blueprints/AI/AI_Character.IsMoving` true _asai_character)
  (`|AIMoveTo` _returnvalue (`NavigationSystem.GetRandomReachablePointInRadius` (`BTFunctionLibrary.GetBlackboardValueAsVector` (`self.LSPoint`)) 100.0) null 20.0
    (:`OnSuccess`
      (`self.FinishExecute` true))
    (:`OnFail`
      (`self.FinishExecute` false))))