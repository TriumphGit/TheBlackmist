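; Behavior tree service that handles aggro detection for AI pawns run by Follower_AI_CON2.
; Each tick it flags combat and sphere-traces the controller's RAggro2 radius, ignoring other AI_Characters, then line-traces to each hit to confirm sight.
; Visible hits set the target, location, last-seen point and SeePlayer blackboard keys; blocked ones clear target, SeePlayer and WantsFire.
; A dead pawn only stops firing.
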(event `self.ReceiveTick`
  (params (OwnerActor :type "Actor Object Reference") (DeltaSeconds :type "Float (single-precision)"))
  (bind _seeplayer (`self.SeePlayer`))
  (bind _returnvalue (`Controller.K2_GetPawn` (`self.AI_CON_Ref`)))
  (bind _returnvalue_2 (`Actor.K2_GetActorLocation` _returnvalue))
  (if (not (!= (`self.AI_CON_Ref`) null))
    (bind _asfollower_ai_con2 (cast `/Game/Blueprints/AI/Follower_AI_CON2` OwnerActor))
    (bind _output_get (set `self.AI_CON_Ref` _asfollower_ai_con2)))
  (bind _outactors (`GameplayStatics.GetAllActorsOfClass` "/Game/Blueprints/AI/AI_Character.AI_Character_C"))
  (bind _asai_character (cast `/Game/Blueprints/AI/AI_Character` _returnvalue))
  (if (`/Game/Blueprints/AI/AI_Character.IsDead` _asai_character)
    (set `/Game/Blueprints/AI/AI_Character.WantsFire` false _asai_character)
    (else
      (set `/Game/Blueprints/AI/Follower_AI_CON2.LocationCombat` _returnvalue_2 _output_get)
      (bind _output_get_2 (set `self.MyLocation` _returnvalue_2))
      (set `/Game/Blueprints/AI/Follower_AI_CON2.IsCombat` true _asfollower_ai_con2)
      (bind (_outhits _returnvalue_3) (`KismetSystemLibrary.SphereTraceMultiForObjects` _output_get_2 (+ _returnvalue_2 (0.0 0.0 15.0)) (`/Game/Blueprints/AI/Follower_AI_CON2.RAggro2` _output_get) (`self.DesiredObjectTypes`) false _outactors "ForDuration"))
      (for _array_element _outhits
        (bind (_bblockinghit _binitialoverlap _time _location _impactpoint _normal _impactnormal _physmat _hitactor) (`GameplayStatics.BreakHitResult` _array_element))
        (bind _outhit (`KismetSystemLibrary.LineTraceSingle` (`self.MyLocation`) (`Actor.K2_GetActorLocation` _hitactor) "TraceTypeQuery2" false _outactors "ForDuration"))
        (bind (_bblockinghit_2 _binitialoverlap_2 _time_2 _location_2 _impactpoint_2 _normal_2 _impactnormal_2 _physmat_2 _hitactor_2) (`GameplayStatics.BreakHitResult` _outhit))
        (if (== _hitactor_2 _hitactor)
          (`BTFunctionLibrary.SetBlackboardValueAsObject` (`self.TargetToFollow`) _hitactor_2)
          (`BTFunctionLibrary.SetBlackboardValueAsVector` (`self.TargetLocation`) (`Actor.K2_GetActorLocation` _hitactor_2))
          (`BTFunctionLibrary.SetBlackboardValueAsVector` (`self.LastSeenPoint`) _location_2)
          (if _returnvalue_3
            (`BTFunctionLibrary.SetBlackboardValueAsBool` _seeplayer true)
            (else
              (`BTFunctionLibrary.SetBlackboardValueAsBool` _seeplayer)))
          (else
            (`BTFunctionLibrary.SetBlackboardValueAsObject` (`self.TargetToFollow`))
            (set `/Game/Blueprints/AI/AI_Character.WantsFire` false _asai_character)
            (if _returnvalue_3
              _
              (else
                _))
            (`BTFunctionLibrary.SetBlackboardValueAsBool` (`self.SeePlayer`))))))))