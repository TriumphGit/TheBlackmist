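; WPRifle is a rifle pickup actor that the player collects with the GrabWeapon input.
; It enables player input on BeginPlay, and its Trigger overlap events toggle CanInteract to gate the grab.
; On a grab it destroys itself, casts the overlapping actor to ThirdPersonCharacter, sets HasRifle, and shows the character's own Weapon component attached to the mesh's back socket.
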(event `self.ReceiveBeginPlay`
  (`self.EnableInput` (`GameplayStatics.GetPlayerController` 0)))

(event `InputAction|GrabWeapon` :consume false
  (params (Key :type "Key Structure" :default "AnyKey"))
  (:`Pressed`
    (if (`self.CanInteract`)
      (`self.K2_DestroyActor`)
      (bind _asthird_person_character (cast `/Game/Character/ThirdPersonCharacter/ThirdPersonCharacter` (stale `self.Trigger.OnComponentBeginOverlap` OtherActor)))
      (bind _output_get (set `/Game/Character/ThirdPersonCharacter/ThirdPersonCharacter.HasRifle` true _asthird_person_character))
      (if _output_get
        (bind _weapon (`/Game/Character/ThirdPersonCharacter/ThirdPersonCharacter.Weapon` _asthird_person_character))
        (`SceneComponent.K2_AttachTo` _weapon (`Character.Mesh` _asthird_person_character) "Back_WeaponSocket" "KeepRelativeOffset" true)
        (`SceneComponent.SetVisibility` _weapon true false)))))

(event `self.Trigger.OnComponentBeginOverlap`
  (params (OtherActor :type "Actor Object Reference") (OtherComp :type "PrimitiveComponent Object Reference") (OtherBodyIndex :type Integer) (bFromSweep :type Boolean) (SweepResult :type "HitResult Structure (by ref)"))
  (set `self.CanInteract` true))

(event `self.Trigger.OnComponentEndOverlap`
  (params (OtherActor :type "Actor Object Reference") (OtherComp :type "PrimitiveComponent Object Reference") (OtherBodyIndex :type Integer))
  (set `self.CanInteract` false))

(event `self.ReceiveTick`
  (params (DeltaSeconds :type "Float (single-precision)")))

(fn `UserConstructionScript`)