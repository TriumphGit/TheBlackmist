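; RifleAmmo is a rifle ammo Blueprint whose graphs capture the owning character's aim direction.
; Its construction script casts the owner to ThirdPersonCharacter and copies AimVec into AmmoDirect.
; Tick only casts the player pawn to that class; nodes for the weapon's AmmoEject socket and for stepping the static mesh along AmmoDirect are unconnected, so these graphs apply no movement.
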(event `self.ReceiveTick`
  (params (DeltaSeconds :type "Float (single-precision)"))
  (bind _asthird_person_character (cast `/Game/Character/ThirdPersonCharacter/ThirdPersonCharacter` (`GameplayStatics.GetPlayerPawn` 0))))

(fn `UserConstructionScript`
  (bind _asthird_person_character (cast `/Game/Character/ThirdPersonCharacter/ThirdPersonCharacter` (`self.GetOwner`)))
  (set `self.AmmoDirect` (`/Game/Character/ThirdPersonCharacter/ThirdPersonCharacter.AimVec` _asthird_person_character)))